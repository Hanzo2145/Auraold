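; Enemy ranged attack Gameplay Ability that fires a projectile at the avatar's combat target.
; On activation it turns the avatar toward the target via CombatInterface and plays a random tagged montage.
; The montage's gameplay event tag triggers the projectile spawn from that montage's socket, using the target's then-current location and a fixed pitch override.
; The ability ends when the montage completes, is interrupted or is cancelled.
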(event `self.K2_ActivateAbility`
  (bind _returnvalue (`self.GetAvatarActorFromActorInfo`))
  (bind (_taggedmontage_montage _taggedmontage_montagetag _taggedmontage_sockettag) (break `TaggedMontage` (`self.TaggedMontage`)))
  (bind _returnvalue_2 (message `EnemyInterface.GetCombatTarget` _returnvalue))
  (bind _ascombat_interface (cast `CombatInterface` _returnvalue))
  (`CombatInterface.UpdatingFacingTarget` _ascombat_interface (`Actor.K2_GetActorLocation` _returnvalue_2))
  (bind _returnvalue_3 (message `CombatInterface.GetTaggedMontages` _returnvalue))
  (bind _output_get (set `self.TaggedMontage` (`self.GetRandomedMontageFromArray` _returnvalue_3)))
  (bind (_montage _montagetag) (break `TaggedMontage` _output_get))
  (`AbilityTask_PlayMontageAndWait.CreatePlayMontageAndWaitProxy` "None" _montage 1.0 "None" false
    (:`then`
      (`AbilityTask_WaitGameplayEvent.WaitGameplayEvent` _montagetag null
        (:`EventReceived`
          (bind _returnvalue_4 (message `EnemyInterface.GetCombatTarget` (`self.GetAvatarActorFromActorInfo`)))
          (`self.SpawnProjectile` (`Actor.K2_GetActorLocation` _returnvalue_4) _taggedmontage_sockettag true 25.0))))
    (:`OnCompleted`
      (`self.K2_EndAbility` :!label _label))
    (:`OnInterrupted`
      (goto _label))
    (:`OnCancelled`
      (goto _label))))