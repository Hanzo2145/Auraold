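; Fire Bolt gameplay ability that casts a projectile at the point under the mouse.
; On activation, a target data task supplies the hit location, and the avatar turns toward it through CombatInterface before playing the cast montage.
; The montage's FireBolt gameplay event times the SpawnProjectile call, after which the ability ends locally.
; Montage completion and interruption are not handled, so only that event ends the ability here.
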(event `self.K2_ActivateAbility`
  (bind (_asynctaskproxy _datahandle) (`TargetDataUnderMouse.CreateTagretDataUnderMouse`)
    (:`ValidData`
      (set `self.Projectile Target Location` (`.ImpactPoint` (`GameplayStatics.BreakHitResult` (`AbilitySystemBlueprintLibrary.GetHitResultFromTargetData` _datahandle))))
      (bind _ascombat_interface (cast `CombatInterface` (`self.GetAvatarActorFromActorInfo`)))
      (`CombatInterface.UpdatingFacingTarget` _ascombat_interface (`self.Projectile Target Location`))
      (`AbilityTask_PlayMontageAndWait.CreatePlayMontageAndWaitProxy` "None" "/Game/Assets/Characters/Aura/Animations/Abilities/AM_Cast_FireBolt.AM_Cast_FireBolt"
        (:`then`
          (`AbilityTask_WaitGameplayEvent.WaitGameplayEvent` (struct :`TagName` "Event.Montage.FireBolt") null
            (:`EventReceived`
              (`self.SpawnProjectile` (`self.Projectile Target Location`))
              (`self.K2_EndAbilityLocally`))))))))